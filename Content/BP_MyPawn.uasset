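; Test pawn that flies relative to the camera via world offsets, with controller look input and button-adjusted, clamped speed.
; On BeginPlay it spawns two BP_MoveActors with different speeds, keeping only the second to call PrintHello and move along its up vector from input axes.
; Movement is not scaled by delta time or swept for collision.
; HelloWorld input prints debug messages, while AxisTest and NewFunction0 are empty.
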(event `self.ReceiveBeginPlay`
  (`|SpawnActorFromClass` "/Game/BP_MoveActor.BP_MoveActor_C" (`KismetMathLibrary.MakeTransform` (0.0 100.0 0.0) (struct)) "Undefined" "OverrideRootScale" null 0.0 250.0 null)
  (bind _returnvalue (`|SpawnActorFromClass` "/Game/BP_MoveActor.BP_MoveActor_C" (`KismetMathLibrary.MakeTransform` (0.0 0.0 0.0)) "Undefined" "OverrideRootScale" null 0.0 600.0 null))
  (bind _output_get (set `self.MoveActor` _returnvalue))
  (`/Game/BP_MoveActor.PrintHello` _output_get))

(event `InputAction|HelloWorld`
  (params (Key :type "Key Structure"))
  (:`Pressed`
    (`KismetSystemLibrary.PrintString` "HelloWorld Pressed" true true (struct :`G` 0.66 :`B` 1.0 :`A` 1.0) 60.0))
  (:`Released`
    (`KismetSystemLibrary.PrintString` "HelloWorld Released" true true (struct :`G` 0.66 :`B` 1.0 :`A` 1.0) 60.0)))

(event `InputAxis|AxisTest`
  (params (AxisValue :type "Float (single-precision)")))

(event `InputAxis|MoveForward`
  (params (AxisValue :type "Float (single-precision)"))
  (`self.K2_AddActorWorldOffset` (* (`self.GetActorForwardVector` (`GameplayStatics.GetPlayerCameraManager` 0)) (* AxisValue (`self.PlayerSpeed`)))))

(event `InputAction|SpeedUp`
  (params (Key :type "Key Structure"))
  (:`Pressed`
    (bind _output_get (set `self.PlayerSpeed` (+ (`self.PlayerSpeed`) 10.0)))
    (if (>= _output_get 100.0)
      (set `self.PlayerSpeed` 100.0))))

(event `InputAction|SpeedDown`
  (params (Key :type "Key Structure"))
  (:`Pressed`
    (bind _output_get (set `self.PlayerSpeed` (- (`self.PlayerSpeed`) 10.0)))
    (if (<= _output_get 10.0)
      (set `self.PlayerSpeed` 10.0))))

(event `InputAxis|MoveRight`
  (params (AxisValue :type "Float (single-precision)"))
  (`self.K2_AddActorWorldOffset` (* (`self.GetActorRightVector` (`GameplayStatics.GetPlayerCameraManager` 0)) (* AxisValue (`self.PlayerSpeed`)))))

(event `InputAxis|LookUp`
  (params (AxisValue :type "Float (single-precision)"))
  (`self.AddControllerPitchInput` AxisValue))

(event `InputAxis|LookRight`
  (params (AxisValue :type "Float (single-precision)"))
  (`self.AddControllerYawInput` AxisValue))

(event `InputAxis|ActorMoveUp`
  (params (AxisValue :type "Float (single-precision)"))
  (bind _moveactor (`self.MoveActor`))
  (`self.K2_AddActorWorldOffset` _moveactor (* (`SceneComponent.GetUpVector` (`/Game/BP_MoveActor.DefaultSceneRoot` _moveactor)) (* AxisValue 30.0)) false false))

(event `InputAxis|ActorMoveDown`
  (params (AxisValue :type "Float (single-precision)"))
  (bind _moveactor (`self.MoveActor`))
  (`self.K2_AddActorWorldOffset` _moveactor (* (`SceneComponent.GetUpVector` (`/Game/BP_MoveActor.DefaultSceneRoot` _moveactor)) (* AxisValue 30.0)) false false))

(fn `NewFunction_0`)

(fn `UserConstructionScript`)