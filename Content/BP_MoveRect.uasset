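; BP_MoveRect moves its Sphere component around a square loop in relative XY space, between zero and DestPos on each axis.
; While IsPlay is set, Tick switches on the MoveType enum and calls the matching directional function.
; Each function offsets the Sphere by Speed scaled by delta time and advances MoveType once it passes its boundary, forming a simple cyclic state machine without clamping at the corners.
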(event `self.ReceiveTick`
  (params (DeltaSeconds :type "Float (single-precision)"))
  (if (`self.IsPlay`)
    (switch `/Game/En_MoveType` (`self.MoveType`)
      (:`NewEnumerator0`
        (`self.MoveRight` DeltaSeconds))
      (:`NewEnumerator6`
        (`self.MoveTop` DeltaSeconds))
      (:`NewEnumerator1`
        (`self.MoveLeft` DeltaSeconds))
      (:`NewEnumerator7`
        (`self.MoveBottom` DeltaSeconds)))))

(fn `MoveBottom`
  (params (DeltaSecond :type "Float (double-precision)"))
  (bind (_relativelocation_x _relativelocation_y) (`KismetMathLibrary.BreakVector` (`SceneComponent.RelativeLocation` (`self.Sphere`))))
  (bind _result (`/Engine/EditorBlueprintResources/StandardMacros.NegateFloat` (* DeltaSecond (`self.Speed`)))
    (:`  `
      (`SceneComponent.K2_AddRelativeLocation` (`self.Sphere`) (`KismetMathLibrary.MakeVector` 0.0 _result) false false)
      (if (< _relativelocation_y 0.0)
        (set `self.MoveType` "NewEnumerator0")))))

(fn `MoveLeft`
  (params (DeltaSecond :type "Float (double-precision)"))
  (bind _relativelocation_x (`KismetMathLibrary.BreakVector` (`SceneComponent.RelativeLocation` (`self.Sphere`))))
  (bind _result (`/Engine/EditorBlueprintResources/StandardMacros.NegateFloat` (* DeltaSecond (`self.Speed`)))
    (:`  `
      (`SceneComponent.K2_AddRelativeLocation` (`self.Sphere`) (`KismetMathLibrary.MakeVector` _result) false false)
      (if (< _relativelocation_x 0.0)
        (set `self.MoveType` "NewEnumerator7")))))

(fn `MoveRight`
  (params (DeltaSecond :type "Float (double-precision)"))
  (bind _relativelocation_x (`KismetMathLibrary.BreakVector` (`SceneComponent.RelativeLocation` (`self.Sphere`))))
  (`SceneComponent.K2_AddRelativeLocation` (`self.Sphere`) (`KismetMathLibrary.MakeVector` (* DeltaSecond (`self.Speed`))) false false)
  (if (> _relativelocation_x (`self.DestPos`))
    (set `self.MoveType` "NewEnumerator6")))

(fn `MoveTop`
  (params (DeltaSecond :type "Float (double-precision)"))
  (bind (_relativelocation_x _relativelocation_y) (`KismetMathLibrary.BreakVector` (`SceneComponent.RelativeLocation` (`self.Sphere`))))
  (`SceneComponent.K2_AddRelativeLocation` (`self.Sphere`) (`KismetMathLibrary.MakeVector` 0.0 (* DeltaSecond (`self.Speed`))) false false)
  (if (> _relativelocation_y (`self.DestPos`))
    (set `self.MoveType` "NewEnumerator1")))

(fn `UserConstructionScript`)